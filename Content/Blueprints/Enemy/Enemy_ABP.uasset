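; Enemy_ABP is the base Actor for space enemies such as meteors and asteroids, handling collisions and death.
; On overlap it ignores projectiles, teleports itself away from other enemies, or damages anything else by a fraction of its own health and destroys itself, also notifying a struck SpaceShip.
; EndPlay notifies the game mode of the kill and spawns a death effect chosen from a class-to-system map.
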(event EventBeginPlay)

(event Collision|EventActorBeginOverlap
  (params (OtherActor :type Actor%20Object%20Reference))
  (bind _returnvalue (Utilities|GetClass OtherActor))
  (bind _returnvalue_2 (Transformation|GetActorLocation OtherActor))
  (bind _self self)
  (bind _returnvalue_3 (Transformation|GetActorLocation _self))
  (if (not (Utilities|ClassIsChildOf _returnvalue "/Game/Blueprints/Projectiles/Projectile_ABP.Projectile_ABP_C"))
    (if (Utilities|ClassIsChildOf _returnvalue "Enemy_ABP_C")
      (Transformation|SetActorLocation (+ (* (Math|Random|RandomFloatinRange 1e+03 2e+03) (Math|Random|RandomUnitVector)) (Transformation|GetActorLocation)) false true)
      (else
        (Utilities|IsValid _self
          (:Is%20Valid
            (bind _outhit (Collision|LineTraceByChannel _returnvalue_3 _returnvalue_2 "TraceTypeQuery1" false 0 "None"))
            (Game|Damage|ApplyPointDamage OtherActor (/ (Variables|/Game/Blueprints/HealthCompnent_BP.HealthCompnent_BP_C|GetHealth (Variables|Default|GetHealthCompnent_BP)) 1e+01) (Math|Vector|GetUnitDirection(Vector) _returnvalue_3 _returnvalue_2) _outhit)
            (if (== (Utilities|GetClass OtherActor) "/Game/Blueprints/SpaceShip.SpaceShip_C")
              (Class|PlayerActionsIBP|KilledEvent(Message) OtherActor (Utilities|GetClass self) "NewEnumerator1"))
            (Actor|DestroyActor _self)))))))

(event EventTick
  (params (DeltaSeconds :type Float%20%28single-precision%29)))

(event EventEndPlay
  (params (EndPlayReason :type EEndPlayReason%20Enum :default "Destroyed"))
  (bind _returnvalue (Transformation|GetActorLocation))
  (bind _map (Utilities|Map|MakeMap "/Game/Blueprints/Enemy/EN_Meteor_BP.EN_Meteor_BP_C" "/Game/Effects/MeteorDies.MeteorDies" "/Game/Blueprints/Enemy/EN_Asteroid_BP.EN_Asteroid_BP_C" "/Game/Effects/AsteroidDies.AsteroidDies"))
  (bind _self self)
  (bind _returnvalue_2 (Utilities|GetClass _self))
  (bind (_value _returnvalue_3) (Utilities|Map|Find _map _returnvalue_2))
  (Development|PrintString (Utilities|String|ToString(Vector) _returnvalue))
  (Class|GamemodeActionsIBP|EnemyKilled(Message) (Game|GetGameMode))
  (if _returnvalue_3
    (Niagara|SpawnSystematLocation _value _returnvalue)))

(fn ConstructionScript)