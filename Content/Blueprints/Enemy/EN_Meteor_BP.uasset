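; Enemy meteor pawn that flies toward the Station actor at a fixed speed.
; On BeginPlay it finds the Station and starts a looping short-interval timer, which repeatedly points the FloatingPawnMovement velocity at the target instead of using Tick.
; The timer clears itself if the meteor is no longer valid.
; No overlap, damage or impact logic is implemented in this graph.
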(event Custom|CustomEvent
  (Utilities|IsValid self
    (:Is%20Valid
      (Variables|/Script/Engine.MovementComponent|SetVelocity (Variables|Default|GetFloatingPawnMovement) (* (Math|Vector|GetUnitDirection(Vector) (Transformation|GetActorLocation self) (Transformation|GetActorLocation (Variables|Default|GetTarget))) 2e+03)))
    (:Is%20Not%20Valid
      (Utilities|Time|ClearandInvalidateTimerbyHandle (Variables|Default|GetTimer)))))

(event EventBeginPlay
  (bind _returnvalue (Actor|GetActorOfClass "/Game/Blueprints/Station.Station_C"))
  (Variables|Default|SetTarget _returnvalue)
  (bind _returnvalue_2 (Utilities|Time|SetTimerbyEvent (delegate Custom|CustomEvent) 0.1 true))
  (Variables|Default|SetTimer _returnvalue_2))

(event Collision|EventActorBeginOverlap
  (params (OtherActor :type Actor%20Object%20Reference)))

(event EventTick
  (params (DeltaSeconds :type Float%20%28single-precision%29)))

(fn ConstructionScript
  (|CallParentFunction))