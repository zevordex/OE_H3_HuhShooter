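; Projectile manager that spawns projectiles either as real actors or as lightweight "hypothetical" struct entries, ticking both on one looping timer.
; Real projectiles run custom tick logic or sweep along their direction, applying point damage and a hit effect before destruction.
; Hypothetical projectiles advance by sphere trace in a map, but hit handling and removal are unimplemented and instanced-mesh rendering is disconnected.
; Live counts print each timer tick.
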(event Custom|CustomEvent
  (bind (_total _hypo _real) (CallFunction|GetCurrentProjectileAmount))
  (bind _realprojectiles_t (Variables|Default|GetRealProjectiles_T))
  (Development|PrintString (Utilities|String|Append "Total: " (Utilities|String|ToString(Integer) _total) " 
Hypo:" (Utilities|String|ToString(Integer) _hypo) " 
Real:" (Utilities|String|ToString(Integer) _real)) true false "(R=1.000000,G=0.000000,B=0.089263,A=1.000000)" 2.0 "ProjCount")
  (Utilities|FlowControl|Sequence
    (:then_0
      (bind _keys (Utilities|Map|Keys (Variables|Default|GetHypoProjectiles_T)))
      (for _array_element _keys
        (CallFunction|TickHypoProjectile (Variables|Default|GetBulletTickrate_T) _array_element)))
    (:then_1
      (for _array_element_2 _realprojectiles_t
        (Utilities|IsValid _array_element_2
          (:Is%20Valid
            (if (Variables|/Game/Blueprints/Projectiles/Projectile_ABP.Projectile_ABP_C|GetCustomTickAction _array_element_2)
              (Default|Ticked _array_element_2 (Variables|Default|GetBulletTickrate_T))
              (else
                (bind (_sweephitresult _returnvalue) (Transformation|SetActorLocation _array_element_2 (+ (* (Variables|/Game/Blueprints/Projectiles/Projectile_ABP.Projectile_ABP_C|GetDirection _array_element_2) 0.02) (Transformation|GetActorLocation _array_element_2)) true false))
                (if _returnvalue
                  (Utilities|IsValid (.HitActor (Collision|BreakHitResult _sweephitresult))
                    (:Is%20Valid
                      (Development|PrintString (Utilities|GetDisplayName (.HitActor (Collision|BreakHitResult _sweephitresult))) false false)
                      (Game|Damage|ApplyPointDamage (.HitActor (Collision|BreakHitResult _sweephitresult)) (Variables|/Game/Blueprints/Projectiles/Projectile_ABP.Projectile_ABP_C|GetDamage _array_element_2) (.TraceStart (Collision|BreakHitResult _sweephitresult)) _sweephitresult 0 (Game|GetInstigator _array_element_2))
                      (Niagara|SpawnSystematLocation "/Game/Effects/BulletHit.BulletHit" (.Location (Collision|BreakHitResult _sweephitresult)))
                      (Actor|DestroyActor _array_element_2)))))))
          (:Is%20Not%20Valid
            (Utilities|Array|RemoveItem _realprojectiles_t _array_element_2)))))))

(event EventBeginPlay
  (Utilities|Time|SetTimerbyEvent (delegate Custom|CustomEvent) (Variables|Default|GetBulletTickrate_T) true))

(event Collision|EventActorBeginOverlap
  (params (OtherActor :type Actor%20Object%20Reference)))

(event EventTick
  (params (DeltaSeconds :type Float%20%28single-precision%29)))

(fn ConstructionScript)

(fn SpawnNewProjectile
  (params (ProjectileClass :type Projectile%20ABP%20Class%20Reference) (SpawnTransform :type Transform) (Instigator :type Pawn%20Object%20Reference) (Lifetime :type Float%20%28double-precision%29) (Direction :type Vector) (Damage :type Float%20%28double-precision%29))
  (bind _returnvalue (Game|SpawnActorfromClass ProjectileClass SpawnTransform "Undefined" "MultiplyWithRoot" 0 Lifetime Direction Damage Instigator))
  (Actor|SetLifeSpan _returnvalue Lifetime)
  (Utilities|Array|Add (Variables|Default|GetRealProjectiles_T) _returnvalue))

(fn SpawnHypotheticalProjectile
  (params (Instigator :type Pawn%20Object%20Reference) (Transform :type Transform) (Direction :type Vector) (LifeTime :type Float%20%28double-precision%29) (Size :type Float%20%28double-precision%29) (Damage :type Float%20%28double-precision%29))
  (bind _result (Math|Integer|IncrementInt (Variables|Default|GetGlobalProjectileCounter_T))
    (:%20%20
      (Utilities|Map|Add (Variables|Default|GetHypoProjectiles_T) _result (Utilities|Struct|MakeSHypoProjectile_old (Actor|GetGameTimeSinceCreation) LifeTime Direction Transform Damage Instigator 0 Size)))))

(fn GetCurrentProjectileAmount
  (bind _hypoprojectiles_t (Variables|Default|GetHypoProjectiles_T))
  (bind _realprojectiles_t (Variables|Default|GetRealProjectiles_T))
  (bind _returnvalue (Utilities|Array|Length _realprojectiles_t))
  (bind _returnvalue_2 (Utilities|Map|Length _hypoprojectiles_t))
  (return (+ _returnvalue_2 _returnvalue) _returnvalue_2 _returnvalue))

(fn TickHypoProjectile
  (params (Delta :type Float%20%28double-precision%29) (ProjectileId :type Integer))
  (bind _hypoprojectiles_t (Variables|Default|GetHypoProjectiles_T))
  (bind (_value _returnvalue) (Utilities|Map|Find _hypoprojectiles_t ProjectileId))
  (bind (_secondstimestamp _lifetime _direction _position _damage _owner _renderid _size) (Utilities|Struct|BreakSHypoProjectile_old _value))
  (bind (_location _rotation _scale) (Math|Transform|BreakTransform _position))
  (bind _returnvalue_2 (* Delta _direction))
  (bind _returnvalue_3 (+ _returnvalue_2 _location))
  (if _returnvalue
    (LocalVariables|SetPrevLoc _location)
    (Collision|SphereTraceByChannel (LocalVariables|GetPrevLoc) _returnvalue_3 _size "TraceTypeQuery3" false 0 "None" true "(R=1.000000,G=0.000000,B=0.000000,A=1.000000)" "(R=0.000000,G=1.000000,B=0.000000,A=1.000000)" 0.2)
    (bind _structout (Utilities|Struct|SetmembersinSHypoProjectile_old _value (Math|Transform|MakeTransform _returnvalue_3 _rotation _scale)))
    (Utilities|Map|Add (Variables|Default|GetHypoProjectiles_T) ProjectileId _structout)))

(fn DestroyHypoProjectile
  (params (Id :type Integer)))