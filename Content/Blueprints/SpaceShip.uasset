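; Player spaceship pawn that flies through a movement component, fires two socket-mounted machine guns and scores kills, with a bonus for rams.
; Mouse and timer-driven roll input turn the spring arm; on authority, Tick eases the hull toward the camera's aim using quaternion rotation and prints debug values.
; Boost also intensifies engine particles and widens light radii.
; Health component events update HUD bars for ship and Station, alongside ammo and score.
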(event Custom|MouseInput_SERVER
  (params (X :type Float%20%28double-precision%29) (Y :type Float%20%28double-precision%29)))

(event Custom|RollEvent
  (bind _springarm (Variables|Default|GetSpringArm))
  (bind _relativerotation (Variables|/Script/Engine.SceneComponent|GetRelativeRotation _springarm))
  (Transformation|SetRelativeRotation _springarm (Math|Rotator|MakeRotator (+ (.roll _relativerotation) (Variables|Default|GetRollStatus)) (.pitch _relativerotation) (.yaw _relativerotation)) false false))

(event Custom|CustomEvent
  (params (Shield :type Float%20%28double-precision%29) (MaxShield :type Float%20%28double-precision%29) (Health :type Float%20%28double-precision%29) (MaxHealth :type Float%20%28double-precision%29))
  (Default|UpdateStationHud (Variables|/Game/Blueprints/UI/MyHUD.MyHUD_C|GetOverlayWidget (Variables|Default|GetAs%20My%20HUD)) Health MaxHealth Shield MaxShield))

(event Custom|CustomEvent_0
  (params (Shield :type Float%20%28double-precision%29) (MaxShield :type Float%20%28double-precision%29) (Health :type Float%20%28double-precision%29) (MaxHealth :type Float%20%28double-precision%29))
  (Default|UpdateShipHud (Variables|/Game/Blueprints/UI/MyHUD.MyHUD_C|GetOverlayWidget (Variables|Default|GetAs%20My%20HUD)) Health MaxHealth Shield MaxShield))

(event Input|EnhancedActionEvents|EnhancedInputActionIA_Mouse
  (params (ActionValue :type Vector%202D%20Structure) (ElapsedSeconds :type Float%20%28double-precision%29) (TriggeredSeconds :type Float%20%28double-precision%29) (InputAction :type Input%20Action%20Object%20Reference :default "/Game/input/Actions/IA_Mouse.IA_Mouse"))
  (bind _returnvalue (Class|FlightQuaterions|EulertoQuaternion (Math|Rotator|MakeRotator 0.0 (.y ActionValue) (.x ActionValue))))
  (Class|FlightQuaterions|AddLocalRotationQuat (Variables|Default|GetSpringArm) _returnvalue))

(event Input|EnhancedActionEvents|EnhancedInputActionIA_debug
  (params (ActionValue :type Boolean) (ElapsedSeconds :type Float%20%28double-precision%29) (TriggeredSeconds :type Float%20%28double-precision%29) (InputAction :type Input%20Action%20Object%20Reference :default "/Game/input/Actions/IA_debug.IA_debug"))
  (:Started
    (Variables|Default|SetVar (not (Variables|Default|GetVar)))))

(event Input|EnhancedActionEvents|EnhancedInputActionIA_Boost
  (params (ActionValue :type Boolean) (ElapsedSeconds :type Float%20%28double-precision%29) (TriggeredSeconds :type Float%20%28double-precision%29) (InputAction :type Input%20Action%20Object%20Reference :default "/Game/input/Actions/IA_Boost.IA_Boost"))
  (bind _pointlight (Variables|Default|GetPointLight))
  (bind _pointlight1 (Variables|Default|GetPointLight1))
  (bind _pointlight2 (Variables|Default|GetPointLight2))
  (bind _pointlight3 (Variables|Default|GetPointLight3))
  (bind _spaceshipmovement (Variables|Default|GetSpaceShipMovement))
  (bind _array (Utilities|Array|MakeArray _pointlight _pointlight1 _pointlight2 _pointlight3))
  (:Triggered
    (Default|SetBoost _spaceshipmovement true)
    (CallFunction|SetEngineBoost (Variables|Default|GetEngine) true)
    (CallFunction|SetEngineBoost (Variables|Default|GetEngine1) true)
    (CallFunction|SetEngineBoost (Variables|Default|GetEngine2) true)
    (CallFunction|SetEngineBoost (Variables|Default|GetEngine3) true)
    (for _array_element _array
      (Rendering|Lighting|SetAttenuationRadius _array_element 2.5e+02)))
  (:Completed
    (Default|SetBoost _spaceshipmovement false)
    (CallFunction|SetEngineBoost (Variables|Default|GetEngine) false)
    (CallFunction|SetEngineBoost (Variables|Default|GetEngine1) false)
    (CallFunction|SetEngineBoost (Variables|Default|GetEngine2) false)
    (CallFunction|SetEngineBoost (Variables|Default|GetEngine3) false)
    (for _array_element_2 _array
      (Rendering|Lighting|SetAttenuationRadius _array_element_2 5e+01))))

(event Input|EnhancedActionEvents|EnhancedInputActionIA_Roll
  (params (ActionValue :type Float%20%28double-precision%29) (ElapsedSeconds :type Float%20%28double-precision%29) (TriggeredSeconds :type Float%20%28double-precision%29) (InputAction :type Input%20Action%20Object%20Reference :default "/Game/input/Actions/IA_Roll.IA_Roll"))
  (:Triggered
    (Variables|Default|SetRollStatus ActionValue))
  (:Started
    (bind _returnvalue (Utilities|Time|SetTimerbyEvent (delegate Custom|RollEvent) 0.016 true))
    (Variables|Default|SetRollTimer _returnvalue))
  (:Completed
    (Utilities|Time|ClearandInvalidateTimerbyHandle (Variables|Default|GetRollTimer))))

(event Input|EnhancedActionEvents|EnhancedInputActionIA_Fire
  (params (ActionValue :type Boolean) (ElapsedSeconds :type Float%20%28double-precision%29) (TriggeredSeconds :type Float%20%28double-precision%29) (InputAction :type Input%20Action%20Object%20Reference :default "/Game/input/Actions/IA_Fire.IA_Fire"))
  (bind _result (Utilities|Set|ToArray (Variables|Default|GetWeapons)))
  (for (_array_element _array_index) _result
    (Default|Fire _array_element)
    (Default|UpdateGunId (Variables|/Game/Blueprints/UI/MyHUD.MyHUD_C|GetOverlayWidget (Variables|Default|GetAs%20My%20HUD)) (Variables|/Game/Blueprints/Guns/Gun_ABP.Gun_ABP_C|GetMagazineCurrent _array_element) (Variables|/Game/Blueprints/Guns/Gun_ABP.Gun_ABP_C|GetMagazine _array_element) _array_index)))

(event Input|EnhancedActionEvents|EnhancedInputActionIA_Move
  (params (ActionValue :type Vector :default "0, 0, 0") (ElapsedSeconds :type Float%20%28double-precision%29) (TriggeredSeconds :type Float%20%28double-precision%29) (InputAction :type Input%20Action%20Object%20Reference :default "/Game/input/Actions/IA_Move.IA_Move"))
  (:Triggered
    (Default|InputVector (Variables|Default|GetSpaceShipMovement) ActionValue))
  (:Completed
    (Default|InputVector (Variables|Default|GetSpaceShipMovement) "0, 0, 0")))

(event EventBeginPlay
  (bind _healthcompnent_bp (Variables|Default|GetHealthCompnent_BP))
  (bind _asflight_gamemode_bp (Utilities|Casting|CastToFlight_Gamemode_BP (Game|GetGameMode)))
  (Variables|Default|SetAs%20Flight%20Gamemode%20BP _asflight_gamemode_bp)
  (bind _asplayer_controller (Utilities|Casting|CastToPlayerController (Pawn|GetController self)))
  (Variables|Default|SetAs%20Player%20Controller _asplayer_controller)
  (Input|AddMappingContext (PlayerController|LocalPlayerSubsystems|GetEnhancedInputLocalPlayerSubsystem _asplayer_controller) "/Game/input/Default_Mapping.Default_Mapping" 0 "(bIgnoreAllPressedKeysUntilRelease=True,bForceImmediately=False,bNotifyUserSettings=False)")
  (CallFunction|PlaceWeapon (Variables|Default|GetGunSocket-1) "/Game/Blueprints/Guns/G_MachineGun_BP.G_MachineGun_BP_C")
  (CallFunction|PlaceWeapon (Variables|Default|GetGunSocket-2) "/Game/Blueprints/Guns/G_MachineGun_BP.G_MachineGun_BP_C" 1)
  (EventDispatchers|BindEventtoStatsUpdate (Variables|Default|GetHealthCompnent_BP) (delegate Custom|CustomEvent_0))
  (bind _asmy_hud (Utilities|Casting|CastToMyHUD (HUD|GetHUD (Variables|Default|GetAs%20Player%20Controller))))
  (bind _output_get (Variables|Default|SetAs%20My%20HUD _asmy_hud))
  (Default|UpdateShipHud (Variables|/Game/Blueprints/UI/MyHUD.MyHUD_C|GetOverlayWidget _output_get) (Variables|/Game/Blueprints/HealthCompnent_BP.HealthCompnent_BP_C|GetHealth _healthcompnent_bp) (Variables|/Game/Blueprints/HealthCompnent_BP.HealthCompnent_BP_C|GetMaxHealth _healthcompnent_bp) (Variables|/Game/Blueprints/HealthCompnent_BP.HealthCompnent_BP_C|GetShield _healthcompnent_bp) (Variables|/Game/Blueprints/HealthCompnent_BP.HealthCompnent_BP_C|GetMaxShield _healthcompnent_bp))
  (bind _returnvalue (Actor|GetActorOfClass "/Game/Blueprints/Station.Station_C"))
  (EventDispatchers|BindEventtoStatsUpdate (Variables|/Game/Blueprints/Station.Station_C|GetHealthCompnent_BP _returnvalue) (delegate Custom|CustomEvent))
  (Default|UpdateStationHud (Variables|/Game/Blueprints/UI/MyHUD.MyHUD_C|GetOverlayWidget (Variables|Default|GetAs%20My%20HUD)) (Variables|/Game/Blueprints/HealthCompnent_BP.HealthCompnent_BP_C|GetHealth (Variables|/Game/Blueprints/Station.Station_C|GetHealthCompnent_BP _returnvalue)) (Variables|/Game/Blueprints/HealthCompnent_BP.HealthCompnent_BP_C|GetMaxHealth (Variables|/Game/Blueprints/Station.Station_C|GetHealthCompnent_BP _returnvalue)) (Variables|/Game/Blueprints/HealthCompnent_BP.HealthCompnent_BP_C|GetShield (Variables|/Game/Blueprints/Station.Station_C|GetHealthCompnent_BP _returnvalue)) (Variables|/Game/Blueprints/HealthCompnent_BP.HealthCompnent_BP_C|GetMaxShield (Variables|/Game/Blueprints/Station.Station_C|GetHealthCompnent_BP _returnvalue)))
  (Class|GamemodeActionsIBP|InitHud(Message) (Game|GetGameMode) (Variables|Default|GetAs%20My%20HUD)))

(event Collision|EventActorBeginOverlap
  (params (OtherActor :type Actor%20Object%20Reference)))

(event EventTick
  (params (DeltaSeconds :type Float%20%28single-precision%29))
  (bind _self self)
  (bind _camera (Variables|Default|GetCamera))
  (bind _springarm (Variables|Default|GetSpringArm))
  (bind _returnvalue (Transformation|GetActorRotation _self))
  (bind _returnvalue_2 (Transformation|GetWorldLocation _camera))
  (bind _returnvalue_3 (Math|Vector|GetForwardVector _camera))
  (bind _relativerotation (Variables|/Script/Engine.SceneComponent|GetRelativeRotation _springarm))
  (bind _returnvalue_4 (* _returnvalue_3 1e+03))
  (bind _returnvalue_5 (+ _returnvalue_2 _returnvalue_4))
  (bind _returnvalue_6 (Math|Rotator|FindLookatRotation _returnvalue_2 _returnvalue_5))
  (bind _returnvalue_7 (Math|Rotator|MakeRotator (.roll _relativerotation) (.pitch _returnvalue_6) (.yaw _returnvalue_6)))
  (bind _returnvalue_8 (Math|Interpolation|RInterpTo _returnvalue _returnvalue_7 DeltaSeconds 3.0))
  (bind (_roll _pitch _yaw) (Math|Rotator|BreakRotator _returnvalue_8))
  (Networking|SwitchHasAuthority
    (:Authority
      (Class|PrimitiveComponent|SetAllPhysicsAngularVelocityinDegrees (Variables|Default|GetBox _self) (Math|Vector|MakeVector 0.0 0.0 0.0) false)
      (Class|FlightQuaterions|SetActorWorldRotationQuat self (Math|Conversions|ToQuaternion(Rotator) (Math|Rotator|MakeRotator _roll _pitch _yaw)))
      (Development|PrintString (Utilities|String|Append "Speed: " (Utilities|String|ToString(Float) (Variables|Default|GetSpeed)) " 
" (Utilities|String|ToString(Rotator) _returnvalue_7) " 
" (Utilities|String|ToString(Rotator) (Variables|/Script/Engine.SceneComponent|GetRelativeRotation (Variables|Default|GetBox))) " 
" (Utilities|String|ToString(Vector) (Transformation|GetVelocity)) " 
" (Utilities|String|ToString(Rotator) (Variables|/Script/Engine.SceneComponent|GetRelativeRotation (Variables|Default|GetSpringArm)))) true false "(R=0.941074,G=0.955806,B=1.000000,A=1.000000)" 2.0 "Log"))))

(event EventKilledEvent
  (params (Who :type Enemy%20ABP%20Class%20Reference) (KillType :type EKillType%20Enum :default "NewEnumerator0"))
  (bind _newscore (Default|AddScore (Variables|Default|GetAs%20Flight%20Gamemode%20BP) (Math|Float|Round (* (.ScoreReward (Utilities|GetClassDefaults Who)) (Utilities|Select :Index KillType :NewEnumerator0 1.0 :NewEnumerator1 1.5)))))
  (Default|UpdateScore (Variables|/Game/Blueprints/UI/MyHUD.MyHUD_C|GetOverlayWidget (Variables|Default|GetAs%20My%20HUD)) _newscore))

(fn ConstructionScript)

(fn PlaceWeapon
  (params (Socket :type Scene%20Component%20Object%20Reference) (WeaponClass :type Gun%20ABP%20Class%20Reference) (Index :type Integer))
  (bind _returnvalue (Game|SpawnActorfromClass WeaponClass (Transformation|GetRelativeTransform Socket) "Undefined" "MultiplyWithRoot" 0 Index self))
  (Transformation|AttachComponentToComponent _returnvalue Socket "None" "SnapToTarget" "SnapToTarget" "KeepWorld" true)
  (Utilities|Set|Add (Variables|Default|GetWeapons) _returnvalue))

(fn SetEngineBoost
  (params (Engine :type Niagara%20Component%20Object%20Reference) (Boost :type Boolean))
  (if Boost
    (Niagara|SetNiagaraVariable(Float) Engine "LifeTime" 0.2)
    (Niagara|SetNiagaraVariable(Float) Engine "SpawnRate" 1e+03)
    (Niagara|SetNiagaraVariable(Vector3) Engine "None" "0.000000,0.000000,1000.000000")
    (else
      (Niagara|SetNiagaraVariable(Float) Engine "LifeTime" 0.1)
      (Niagara|SetNiagaraVariable(Float) Engine "SpawnRate" 1e+02)
      (Niagara|SetNiagaraVariable(Vector3) Engine "None" "0.000000,0.000000,100.000000"))))