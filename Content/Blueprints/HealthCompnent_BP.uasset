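; Health component that gives its owning actor health plus a regenerating shield, with game-ending death for the Station and SpaceShip.
; A looping timer refills the shield up to its maximum.
; Damage from non-ignored causer classes hits shield first, without overflow into health, then broadcasts damage and stat updates.
; Lethal damage reports Enemy_ABP kills to the causer, then quits the game for Station or SpaceShip owners and destroys others.
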(event Custom|OnTakeAnyDamage_Event
  (params (DamagedActor :type Actor%20Object%20Reference) (Damage :type Float%20%28single-precision%29) (DamageType :type Damage%20Type%20Object%20Reference) (InstigatedBy :type Controller%20Object%20Reference) (DamageCauser :type Actor%20Object%20Reference))
  (bind _owner (Variables|Default|GetOwner))
  (bind _returnvalue (Utilities|GetClass _owner))
  (if (not (Utilities|Array|ContainsItem (Variables|Default|GetIgnoreFrom) (Utilities|GetClass DamageCauser)))
    (Utilities|IsValid (Variables|Default|GetOwner)
      (:Is%20Valid
        (if (> (Variables|Default|GetShield) 0.0)
          (Variables|Default|SetShield (- (Variables|Default|GetShield) Damage))
          (Default|CallDamageRecieve (Variables|Default|GetOwner) Damage DamageType InstigatedBy DamageCauser (Variables|Default|GetShield) (Variables|Default|GetMaxShield) (Variables|Default|GetHealth) (Variables|Default|GetMaxHealth) :!label _label)
          (Default|CallStatsUpdate (Variables|Default|GetShield) (Variables|Default|GetMaxShield) (Variables|Default|GetHealth) (Variables|Default|GetMaxHealth))
          (elif (<= (- (Variables|Default|GetHealth) Damage) 0.0)
            (bind _asenemy_abp (Utilities|Casting|CastToEnemy_ABPClass _returnvalue)
              (:then
                (Class|PlayerActionsIBP|KilledEvent(Message) DamageCauser _asenemy_abp "NewEnumerator0"))
              (:CastFailed
                _))
            (if (or (== _returnvalue "/Game/Blueprints/Station.Station_C") (== _returnvalue "/Game/Blueprints/SpaceShip.SpaceShip_C"))
              (Game|QuitGame 0 "Quit" false)
              (else
                (Actor|DestroyActor _owner)))
            (else
              (Variables|Default|SetHealth (- (Variables|Default|GetHealth) Damage))
              (goto _label))))))))

(event Custom|CustomEvent
  (if (>= (+ (Variables|Default|GetShieldRegen) (Variables|Default|GetShield)) (Variables|Default|GetMaxShield))
    (Variables|Default|SetShield (Variables|Default|GetMaxShield))
    (else
      (Variables|Default|SetShield (+ (Variables|Default|GetShieldRegen) (Variables|Default|GetShield)))))
  (Default|CallStatsUpdate (Variables|Default|GetShield) (Variables|Default|GetMaxShield) (Variables|Default|GetHealth) (Variables|Default|GetMaxHealth)))

(event EventBeginPlay
  (bind _returnvalue (Components|GetOwner))
  (Utilities|IsValid _returnvalue
    (:Is%20Valid
      (bind _output_get (Variables|Default|SetOwner _returnvalue))
      (EventDispatchers|AssignOnTakeAnyDamage _output_get (delegate Custom|OnTakeAnyDamage_Event))
      (if (> (Variables|Default|GetShieldRegenInterval) 0.0)
        (Utilities|Time|SetTimerbyEvent (delegate Custom|CustomEvent) (Variables|Default|GetShieldRegenInterval) true)))))

(event EventTick
  (params (DeltaSeconds :type Float%20%28single-precision%29)))