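; Enemy spawner Blueprint that spawns waves of enemies at random distant points around the world origin.
; RunWave picks one random 3D anchor per wave, then spawns each entry's count of its enemy class at random radial offsets from that anchor, drawing debug lines.
; A separate custom event spawns a single meteor at a random distant point, but its looping timer setup is unconnected, and Init is empty.
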(event Custom|Init)

(event Custom|CustomEvent
  (bind _output_get (Variables|Default|SetRandomSpawnPos (* (Math|Random|RandomFloatinRange 3e+04 9e+04) (Math|Random|RandomUnitVector))))
  (Rendering|Debug|DrawDebugLine "0, 0, 0" _output_get "(R=1.000000,G=0.821264,B=0.000000,A=1.000000)" 5.0 0.0)
  (Game|SpawnActorfromClass "/Game/Blueprints/Enemy/EN_Meteor_BP.EN_Meteor_BP_C" (Math|Conversions|ToTransform(Vector) _output_get) "Undefined" "MultiplyWithRoot" 0 "0.000000,0.000000,0.000000" 0))

(event Custom|RunWave
  (params (WaveObject :type S%20Wave%20Struct%20Structure))
  (Variables|Default|SetRandomSpawnPos (* (Math|Random|RandomFloatinRange 5e+04 9e+04) (Math|Random|RandomUnitVector)))
  (for _array_element (Utilities|Struct|BreakSWaveStruct WaveObject)
    (for _index (range 1 (.Count (Utilities|Struct|BreakSWaveEnemyData _array_element)))
      (bind _output_get (Variables|Default|SetMoreRandomSpawnPos (+ (* (Math|Random|RandomFloatinRange (.SpawRadiusMin (Utilities|Struct|BreakSWaveEnemyData _array_element)) (.SpawnRadiusMax (Utilities|Struct|BreakSWaveEnemyData _array_element))) (Math|Random|RandomUnitVector)) (Variables|Default|GetRandomSpawnPos))))
      (Rendering|Debug|DrawDebugLine "0, 0, 0" _output_get "(R=1.000000,G=0.821264,B=0.000000,A=1.000000)" 5.0 0.0)
      (Game|SpawnActorfromClass (.EnemyClass (Utilities|Struct|BreakSWaveEnemyData _array_element)) (Math|Conversions|ToTransform(Vector) _output_get) "AdjustIfPossibleButAlwaysSpawn" "MultiplyWithRoot" 0 "0.000000,0.000000,0.000000" 0))))

(event EventBeginPlay)

(event Collision|EventActorBeginOverlap
  (params (OtherActor :type Actor%20Object%20Reference)))

(event EventTick
  (params (DeltaSeconds :type Float%20%28single-precision%29)))

(fn ConstructionScript)