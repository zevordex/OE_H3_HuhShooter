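; Game mode for a flight game that runs enemy waves and tracks score and enemy count.
; BeginPlay spawns the projectile manager and enemy spawner, then starts the game after a short delay.
; When the last enemy dies it runs the next authored wave, or generates meteor and asteroid waves scaled by wave number once those run out.
; It pushes wave, enemy and gun ammo updates to the HUD's overlay widget.
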(event Custom|RunNextWave
  (bind _hud (Variables|Default|GetHud))
  (bind _result (Math|Integer|IncrementInt (Variables|Default|GetCurrentWave))
    (:%20%20
      (bind _sum (CallFunction|TotalEnemiesinWave (Utilities|Array|Get(acopy) (Variables|Default|GetWaves) _result)))
      (Variables|Default|SetTotalEnemies (+ _sum (Variables|Default|GetTotalEnemies)))
      (Default|RunWave (Variables|Default|GetEnemySpawner) (Utilities|Array|Get(acopy) (Variables|Default|GetWaves) _result))
      (Utilities|IsValid _hud
        (:Is%20Valid
          (Default|UpdateGameStats (Variables|/Game/Blueprints/UI/MyHUD.MyHUD_C|GetOverlayWidget _hud) (Variables|Default|GetCurrentWave) (Variables|Default|GetTotalEnemies)))))))

(event Custom|CustomEvent
  (CallFunction|StartGame))

(event EventBeginPlay
  (bind _returnvalue (Game|SpawnActorfromClass "/Game/Blueprints/ProjectileManager_BP.ProjectileManager_BP_C" (Math|Transform|MakeTransform "0, 0, 0" "0, 0, 0" "1.000000,1.000000,1.000000") "Undefined" "MultiplyWithRoot" 0 0))
  (Variables|Default|SetProjectileManager _returnvalue)
  (bind _returnvalue_2 (Game|SpawnActorfromClass "/Game/Blueprints/EnemySpawner_BP.EnemySpawner_BP_C" (Math|Transform|MakeTransform "0, 0, 0" "0, 0, 0" "1.000000,1.000000,1.000000") "Undefined" "MultiplyWithRoot" 0 0))
  (Variables|Default|SetEnemySpawner _returnvalue_2)
  (Utilities|Time|SetTimerbyEvent (delegate Custom|CustomEvent) 5.0))

(event EventTick
  (params (DeltaSeconds :type Float%20%28single-precision%29)))

(event EventEnemyKilled
  (bind _hud (Variables|Default|GetHud))
  (bind _result (Math|Integer|DecrementInt (Variables|Default|GetTotalEnemies))
    (:%20%20
      (Development|PrintString (Utilities|String|ToString(Integer) _result))
      (if (== (Variables|Default|GetTotalEnemies) 0)
        (if (Utilities|Array|IsValidIndex (Variables|Default|GetWaves) (+ (Variables|Default|GetCurrentWave) 1))
          (CallFunction|RunNextWave)
          (else
            (bind _result_2 (Math|Integer|IncrementInt (Variables|Default|GetCurrentWave))
              (:%20%20
                (bind _swavestruct (CallFunction|CreateRandomWave _result_2))
                (CallFunction|RunWaveObject _swavestruct))))))
      (Utilities|IsValid _hud
        (:Is%20Valid
          (Default|UpdateGameStats (Variables|/Game/Blueprints/UI/MyHUD.MyHUD_C|GetOverlayWidget _hud) (Variables|Default|GetCurrentWave) (Variables|Default|GetTotalEnemies)))))))

(event EventInitHud
  (params (Hud :type My%20HUD%20Object%20Reference))
  (Variables|Default|SetHud Hud))

(event EventGunReload
  (params (S1Ammo :type Integer) (S1AmmoMax :type Integer) (Index :type Integer))
  (bind _hud (Variables|Default|GetHud))
  (Utilities|IsValid _hud
    (:Is%20Valid
      (Default|UpdateGunId (Variables|/Game/Blueprints/UI/MyHUD.MyHUD_C|GetOverlayWidget _hud) S1Ammo S1AmmoMax Index))))

(fn ConstructionScript)

(fn StartGame
  (Variables|Default|SetScore 0)
  (Default|Init (Variables|Default|GetEnemySpawner))
  (CallFunction|RunNextWave))

(fn AddScore
  (params (Score :type Integer))
  (bind _output_get (Variables|Default|SetScore (+ Score (Variables|Default|GetScore))))
  (return _output_get))

(fn CreateRandomWave
  (params (WaveNumber :type Integer))
  (if (> WaveNumber 10)
    (return (Utilities|Struct|MakeSWaveStruct (Utilities|Array|MakeArray (Utilities|Struct|MakeSWaveEnemyData "/Game/Blueprints/Enemy/EN_Meteor_BP.EN_Meteor_BP_C" WaveNumber 4e+03 8e+03) (Utilities|Struct|MakeSWaveEnemyData "/Game/Blueprints/Enemy/EN_Asteroid_BP.EN_Asteroid_BP_C" (Math|Integer|Clamp(Integer) (- WaveNumber 10) 0 30) 4e+03 8e+03))))
    (else
      (return (Utilities|Struct|MakeSWaveStruct (Utilities|Array|MakeArray (Utilities|Struct|MakeSWaveEnemyData "/Game/Blueprints/Enemy/EN_Meteor_BP.EN_Meteor_BP_C" (Math|Integer|Clamp(Integer) (* WaveNumber 2) 0 30) 4e+03 8e+03)))))))

(fn RunWaveObject
  (params (Swave :type S%20Wave%20Struct%20Structure))
  (bind _hud (Variables|Default|GetHud))
  (Math|Integer|IncrementInt (Variables|Default|GetCurrentWave)
    (:%20%20
      (bind _sum (CallFunction|TotalEnemiesinWave Swave))
      (Variables|Default|SetTotalEnemies (+ (Variables|Default|GetTotalEnemies) _sum))
      (Default|RunWave (Variables|Default|GetEnemySpawner) Swave)
      (Utilities|IsValid _hud
        (:Is%20Valid
          (Default|UpdateGameStats (Variables|/Game/Blueprints/UI/MyHUD.MyHUD_C|GetOverlayWidget _hud) (Variables|Default|GetCurrentWave) (Variables|Default|GetTotalEnemies)))))))

(fn TotalEnemiesinWave
  (params (SWave :type S%20Wave%20Struct%20Structure))
  (for _array_element (Utilities|Struct|BreakSWaveStruct SWave)
    (LocalVariables|SetTemp (+ (LocalVariables|GetTemp) (.Count (Utilities|Struct|BreakSWaveEnemyData _array_element)))))
  (return (LocalVariables|GetTemp)))