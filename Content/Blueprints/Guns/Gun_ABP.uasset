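; Base gun Actor Blueprint that handles fire rate, magazine count and automatic reloading.
; Fire is gated by cooldown and reload flags, calls the empty DoFire event as a hook for the actual shot, then decrements the magazine.
; Timers drive the cooldown and the reload on an empty magazine.
; Reload completion refills the magazine and reports ammo and gun index to the GameMode.
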(event Custom|DoFire)

(event Custom|onReload
  (Variables|Default|SetReloading false)
  (bind _output_get (Variables|Default|SetMagazineCurrent (Variables|Default|GetMagazine)))
  (Class|GamemodeActionsIBP|GunReload(Message) (Game|GetGameMode) _output_get (Variables|Default|GetMagazine) (Variables|Default|GetIndex)))

(event Custom|onCDExpired
  (Variables|Default|SetinCD false))

(event EventBeginPlay)

(event Collision|EventActorBeginOverlap
  (params (OtherActor :type Actor%20Object%20Reference)))

(event EventTick
  (params (DeltaSeconds :type Float%20%28single-precision%29)))

(fn ConstructionScript)

(fn Fire
  (if (and (not (Variables|Default|GetinCD)) (not (Variables|Default|GetReloading)))
    (Variables|Default|SetinCD true)
    (CallFunction|DoFire)
    (Utilities|FlowControl|Sequence
      (:then_0
        (Utilities|Time|SetTimerbyEvent (EventDispatchers|CreateEvent :!event Custom|onCDExpired) (Variables|Default|GetFireCD)))
      (:then_1
        (bind _output_get (Variables|Default|SetMagazineCurrent (- (Variables|Default|GetMagazineCurrent) 1)))
        (if (< _output_get 1)
          (Variables|Default|SetReloading true)
          (Utilities|Time|SetTimerbyEvent (EventDispatchers|CreateEvent :!event Custom|onReload) (Variables|Default|GetReloadDuration)))))))