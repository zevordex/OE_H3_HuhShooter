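; Machine gun actor that fires bullet projectiles through the flight game mode's shared projectile manager.
; BeginPlay caches the Flight game mode, and DoFire asks its ProjectileManager to spawn a bullet just ahead of the gun with a fixed lifetime and the gun's damage.
; Spawn position and bullet direction both add the instigator's velocity, so shots inherit the shooter's motion.
; An unconnected hypothetical-projectile spawn remains unused.
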(event EventBeginPlay
  (|CallParentFunction)
  (bind _asflight_gamemode_bp (Utilities|Casting|CastToFlight_Gamemode_BP (Game|GetGameMode)))
  (Variables|Default|SetAs%20Flight%20Gamemode%20BP _asflight_gamemode_bp))

(event Collision|EventActorBeginOverlap
  (params (OtherActor :type Actor%20Object%20Reference))
  (|CallParentFunction OtherActor) ; This node is disabled and will not be called.\nDrag off pins to build functionality.
)

(event EventTick
  (params (DeltaSeconds :type Float%20%28single-precision%29))
  (|CallParentFunction DeltaSeconds) ; This node is disabled and will not be called.\nDrag off pins to build functionality.
)

(event EventDoFire
  (bind _returnvalue (Game|GetInstigator))
  (bind _self self)
  (bind _returnvalue_2 (Transformation|GetVelocity _returnvalue))
  (bind _returnvalue_3 (Transformation|GetActorTransform _self))
  (Default|SpawnNewProjectile (Variables|/Game/Blueprints/Flight_Gamemode_BP.Flight_Gamemode_BP_C|GetProjectileManager (Variables|Default|GetAs%20Flight%20Gamemode%20BP)) "/Game/Blueprints/Projectiles/P_Bullet_BP.P_Bullet_BP_C" (Math|Transform|MakeTransform (+ (+ (* (Transformation|GetActorForwardVector _self) 1e+02) (.location _returnvalue_3)) (* _returnvalue_2 0.04)) (.rotation _returnvalue_3) (.scale _returnvalue_3)) _returnvalue 5.0 (+ _returnvalue_2 (* (Transformation|GetActorForwardVector _self) 1e+04)) (Variables|Default|GetDamage)))

(fn ConstructionScript
  (|CallParentFunction))