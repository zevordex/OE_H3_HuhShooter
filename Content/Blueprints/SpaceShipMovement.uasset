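; Movement component for a SpaceShip owner, providing physics thrust, roll and a forward boost.
; InputVector calls DoMovement only with authority (remote just debug-prints), turning thresholded axis input into per-axis power, rotated to ship orientation and applied to its Box as an acceleration force.
; InputRotate sets roll directly through a quaternion, while SetBoost scales forward thrust.
; The MoveTick timer is unconnected and InputVector_SERVER is empty.
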(event Custom|InputVector_SERVER)

(event Custom|MoveTick
  (CallFunction|DoMovement (Variables|Default|GetCurrentMovementVector)))

(event EventBeginPlay
  (bind _asspace_ship (Utilities|Casting|CastToSpaceShip (Components|GetOwner)))
  (Variables|Default|SetAs%20Space%20Ship _asspace_ship))

(event EventTick
  (params (DeltaSeconds :type Float%20%28single-precision%29)))

(fn InputVector
  (params (Vector :type Vector))
  (Networking|SwitchHasAuthority
    (:Authority
      (CallFunction|DoMovement Vector))
    (:Remote
      (Development|PrintString "Hello" true true "(R=1.000000,G=0.000000,B=0.041096,A=1.000000)"))))

(fn DoMovement
  (params (Vector :type Vector))
  (bind (_value_a _value_b) (Utilities|GreaterLessBoolean (.z Vector) 0.5 -0.5))
  (bind (_value_a_2 _value_b_2) (Utilities|GreaterLessBoolean (.x Vector) 0.5 -0.5))
  (bind (_value_a_3 _value_b_3) (Utilities|GreaterLessBoolean (.y Vector) 0.5 -0.5))
  (bind _verticalpower (Variables|Default|GetVerticalPower))
  (bind _horizontalpower (Variables|Default|GetHorizontalPower))
  (bind _as_space_ship (Variables|Default|GetAs%20Space%20Ship))
  (bind _box (Variables|/Game/Blueprints/SpaceShip.SpaceShip_C|GetBox _as_space_ship))
  (Utilities|IsValid (Variables|Default|GetAs%20Space%20Ship)
    (:Is%20Valid
      (Utilities|FlowControl|Sequence
        (:then_0
          (LocalVariables|SetMovementVector (+ (Utilities|SelectVectorTwice _value_a_2 _value_b_2 (Math|Vector|MakeVector (* (Variables|Default|GetForwardPower) (/ (Variables|Default|GetCurrentBoost) 1e+02)) 0.0 0.0) (Math|Vector|MakeVector (CallFunction|*-1 (Variables|Default|GetBackwardPower)) 0.0 0.0)) (LocalVariables|GetMovementVector))))
        (:then_1
          (LocalVariables|SetMovementVector (+ (Utilities|SelectVectorTwice _value_a_3 _value_b_3 (Math|Vector|MakeVector 0.0 _horizontalpower 0.0) (Math|Vector|MakeVector 0.0 (CallFunction|*-1 _horizontalpower) 0.0)) (LocalVariables|GetMovementVector))))
        (:then_2
          (LocalVariables|SetMovementVector (+ (Utilities|SelectVectorTwice _value_a _value_b (Math|Vector|MakeVector 0.0 0.0 _verticalpower) (Math|Vector|MakeVector 0.0 0.0 (CallFunction|*-1 _verticalpower))) (LocalVariables|GetMovementVector)))
          (Physics|AddForce _box (Math|Vector|RotateVector (LocalVariables|GetMovementVector) (Transformation|GetActorRotation _as_space_ship)) "None" true)
          (Development|PrintString (Utilities|String|ToString(Float) (Math|Vector|VectorLength (Transformation|GetComponentVelocity _box))) true false "(R=1.000000,G=0.920735,B=0.000000,A=1.000000)" 2.0 "Vel"))))))

(fn InputRotate
  (params (Direction :type Float%20%28double-precision%29))
  (bind _as_space_ship (Variables|Default|GetAs%20Space%20Ship))
  (bind _returnvalue (Transformation|GetActorRotation _as_space_ship))
  (bind (_roll _pitch _yaw) (Math|Rotator|BreakRotator _returnvalue))
  (Class|FlightQuaterions|SetActorWorldRotationQuat _as_space_ship (Math|Conversions|ToQuaternion(Rotator) (Math|Rotator|MakeRotator (+ (* (Variables|Default|GetRollPower) (Math|Float|Clamp(Float) Direction -1.0)) _roll) _pitch _yaw))))

(fn SetBoost
  (params (NewBoost :type Boolean))
  (if NewBoost
    (Variables|Default|SetCurrentBoost (Variables|Default|GetBoost%25))
    (else
      (Variables|Default|SetCurrentBoost 1e+02))))